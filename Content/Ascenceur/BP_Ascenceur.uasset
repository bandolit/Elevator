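; Elevator actor that starts at a random floor from its Etages height list, with its linked buttons attached to the moving cabin.
; Activate moves the cabin to the requested floor at constant speed, ignoring movement requests while moving, then opens the doors.
; A timeline slides the two doors apart; CloseDoor reverses it, but door positions update only while IsClosing is false.
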(event `self.ReceiveBeginPlay`
  (bind _ascenceur (`self.Ascenceur`))
  (bind _etages (`self.Etages`))
  (bind (_relativelocation_x _relativelocation_y) (`KismetMathLibrary.BreakVector` (`SceneComponent.RelativeLocation` _ascenceur)))
  (for _array_element (`self.Boutons`)
    (`SceneComponent.K2_AttachToComponent` (`Actor.RootComponent` _array_element) (`self.Ascenceur`) "None" "KeepWorld" "KeepWorld" "KeepRelative" true))
  (`SceneComponent.K2_SetRelativeLocation` _ascenceur (`KismetMathLibrary.MakeVector` _relativelocation_x _relativelocation_y (`|GetArrayItem` _etages (`KismetMathLibrary.RandomInteger` (`KismetArrayLibrary.Array_Length` _etages)))) false false))

(event `/Game/Ascenceur/BPI_Activate.Activate`
  (params (Etage :type Integer))
  (bind _ascenceur (`self.Ascenceur`))
  (bind _output (`|GetArrayItem` (`self.Etages`) Etage))
  (bind (_relativelocation_x _relativelocation_y) (`KismetMathLibrary.BreakVector` (`SceneComponent.RelativeLocation` _ascenceur)))
  (set `self.Current_Stage` Etage)
  (if (not (`self.isMoving`))
    (set `self.isMoving` true)
    (`KismetSystemLibrary.MoveComponentTo` _ascenceur (`KismetMathLibrary.MakeVector` _relativelocation_x _relativelocation_y _output) (struct) false false (/ (`KismetMathLibrary.Vector_Distance` (`KismetMathLibrary.MakeVector` 0.0 0.0 _output) (`SceneComponent.RelativeLocation` _ascenceur)) 200.0))
    (`self.Open door`)
    (set `self.isMoving` false)))

(event `Open door`
  (set `self.isClosing` false)
  (bind (_direction _newtrack_0) (`Timeline|Timeline` :!label _label)
    (:`Update`
      (if (not (`self.isClosing`))
        (bind _returnvalue (`KismetMathLibrary.Lerp` 0.0 86.5 _newtrack_0))
        (`SceneComponent.K2_SetRelativeLocation` (`self.R_Door`) (`KismetMathLibrary.MakeVector` _returnvalue) false false)
        (`SceneComponent.K2_SetRelativeLocation` (`self.L_Door`) (`KismetMathLibrary.MakeVector` (* _returnvalue -1.0)) false false)))))

(event `/Game/Ascenceur/BPI_CloseDoor.CloseDoor`
  (set `self.isClosing` true)
  (goto _label :!via `Reverse`))

(fn `UserConstructionScript`)