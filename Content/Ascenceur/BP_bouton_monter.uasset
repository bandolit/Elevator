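; BP_bouton_monter is an interactable elevator up button.
; On Interact it sends its Etage floor value to the referenced Ascenseur through ActivateMessage, then calls CloseDoorMessage on it.
; An unconnected leftover, marked useless, would toggle its BoutonON state in sync with the first BP_bouton_descendre found in the level.
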(event `/Game/Ascenceur/BPI_interact.Interact`
  (bind _ascenseur (`self.Ascenseur`))
  (message `/Game/Ascenceur/BPI_Activate.Activate` _ascenseur (`self.Etage`))
  (message `/Game/Ascenceur/BPI_CloseDoor.CloseDoor` _ascenseur))

(fn `UserConstructionScript`)